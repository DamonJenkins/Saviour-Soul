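; GInstance, apparently the game instance, tallies spirits and ends the level once all are resolved.
; Events increment the total, saved and lost counts, and ResetValues zeroes all three.
; Saving or losing a spirit runs a shared check of saved plus lost against the total.
; On a match, it copies the score from the first GrimReaper actor into PlrScore, removes all widgets and opens the EndScreen level.
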(event `IncreaseSpiritCount`
  (`/Engine/EditorBlueprintResources/StandardMacros.IncrementInt` (`self.SpiritCount`)))

(event `SaveSpirit`
  (bind _result (`/Engine/EditorBlueprintResources/StandardMacros.IncrementInt` (`self.SavedSpirits`))
    (:`  `
      (if (== (+ _result (stale `LoseSpirit` _result)) (`self.SpiritCount`)) :!label _label
        (bind _outactors (`GameplayStatics.GetAllActorsOfClass` "/Game/Blueprints/GrimReaper.GrimReaper_C"))
        (set `self.PlrScore` (`/Game/Blueprints/GrimReaper.Score` (`|GetArrayItem` _outactors)))
        (`WidgetLayoutLibrary.RemoveAllWidgets`)
        (`GameplayStatics.OpenLevel` "EndScreen")))))

(event `LoseSpirit`
  (bind _result (`/Engine/EditorBlueprintResources/StandardMacros.IncrementInt` (`self.LostSpirits`))
    (:`  `
      (goto _label))))

(event `ResetValues`
  (set `self.SpiritCount` 0)
  (set `self.SavedSpirits` 0)
  (set `self.LostSpirits` 0))