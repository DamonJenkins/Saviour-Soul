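; Player Grim Reaper that turns toward the mouse cursor, swings a scythe and casts two swappable abilities.
; Tick drives the curve-based swing and its damage collider, and aims via ray-to-ground-plane math unless the CameraVolume is on its spline.
; Abilities are constructed objects, starting with Dash, cast at a traced cursor point with cooldowns.
; It also handles the health HUD, paused death and ability-choice screens, and a box-overlap "cone" target query.
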(event `self.ReceiveBeginPlay`
  (bind _returnvalue (`GameplayStatics.GetPlayerController` 0))
  (set `PlayerController.bShowMouseCursor` true _returnvalue)
  (bind _returnvalue_2 (`|CreateWidget` "/Game/Blueprints/HealthWidget.HealthWidget_C" _returnvalue))
  (`UserWidget.AddToViewport` _returnvalue_2 0)
  (`DamageComponent.SetHealth` (`self.DmgComponent`) (`self.MaxHealth`))
  (bind _returnvalue_3 (`GameplayStatics.GetActorOfClass` "/Game/Blueprints/cameraVolume.cameraVolume_C"))
  (set `self.cameraVolume` _returnvalue_3)
  (`self.Set Ability One` "/Game/Abilities/DashAbility.DashAbility_C"))

(event `self.ReceiveTick`
  (params (DeltaSeconds :type "Float (single-precision)"))
  (bind _swingtimer (`self.SwingTimer`))
  (bind _capsulecomponent (`self.CapsuleComponent`))
  (bind (_worldlocation _worlddirection) (`PlayerController.DeprojectMousePositionToWorld` (`GameplayStatics.GetPlayerController` 0)))
  (bind (_returnvalue_roll _returnvalue_pitch _returnvalue_yaw) (`KismetMathLibrary.BreakRotator` (`KismetMathLibrary.FindLookAtRotation` (`SceneComponent.K2_GetComponentLocation` _capsulecomponent) (- (`KismetMathLibrary.MakeVector` (.x _worldlocation) (.y _worldlocation) (.z _worldlocation)) (* (`KismetMathLibrary.MakeVector` (.x _worlddirection) (.y _worlddirection) (.z _worlddirection)) (/ (.z _worldlocation) (.z _worlddirection)))))))
  (`PrimitiveComponent.SetCollisionEnabled` (`self.ScytheCollider`) (select `bool` (`self.Swinging`) :`false` "NoCollision" :`true` "QueryOnly" :!type "ECollisionEnabled Enum"))
  (if (`self.Swinging`)
    (if (>= _swingtimer 1.0)
      (set `self.SwingTimer` 0.0)
      (set `self.Swinging` false)
      (else
        (bind _output_get (set `self.SwingTimer` (+ _swingtimer DeltaSeconds)))
        (`SceneComponent.K2_SetRelativeRotation` (`self.ScytheParent`) (* (`KismetMathLibrary.MakeRotator` 80.0 -80.0 -90.0) (`CurveFloat.GetFloatValue` (`self.SwingCurve`) _output_get)) false false))))
  (if (not (`/Game/Blueprints/cameraVolume.onSpline` (`self.cameraVolume`)))
    (`SceneComponent.K2_SetWorldRotation` _capsulecomponent (`KismetMathLibrary.MakeRotator` 0.0 0.0 _returnvalue_yaw) false false)))

(event `InputAction|Attack`
  (params (Key :type "Key Structure"))
  (:`Pressed`
    (if (not (`self.Swinging`))
      (set `self.Swinging` true)
      (`GameplayStatics.PlaySound2D` "/Game/Sound/scytheSwing.scytheSwing" 0.1 1.0 0.0 null null))))

(event `self.ScytheCollider.OnComponentBeginOverlap`
  (params (OverlappedComponent :type "PrimitiveComponent Object Reference") (OtherActor :type "Actor Object Reference") (OtherComp :type "PrimitiveComponent Object Reference") (OtherBodyIndex :type Integer) (bFromSweep :type Boolean) (SweepResult :type "HitResult Structure (by ref)"))
  (bind _returnvalue (`self.GetComponentByClass` OtherActor "/Script/DeathIsTheBeginning.DamageComponent"))
  (`/Engine/EditorBlueprintResources/StandardMacros.IsValid` _returnvalue
    (:`Is Valid`
      (`DamageComponent.Damage` _returnvalue (`self.SwingDamage`) "Good"))))

(event `InputAction|Ability1`
  (params (Key :type "Key Structure"))
  (bind _abilityone (`self.AbilityOne`))
  (:`Pressed`
    (if (`self.CanUseAb1`)
      (bind (_outhit_location _validlocation) (`self.GetMousePositionOnGround`))
      (`/Engine/EditorBlueprintResources/StandardMacros.IsValid` _abilityone
        (:`Is Valid`
          (`/Game/Abilities/AbilityBase.Cast` _abilityone (`self.K2_GetActorLocation` self) _outhit_location _validlocation (0.0 0.0 0.0) false)
          (set `self.CanUseAb1` false)
          (`KismetSystemLibrary.Delay` (`/Game/Abilities/AbilityBase.Cooldown` _abilityone))
          (set `self.CanUseAb1` true))))))

(event `InputAction|Ability2`
  (params (Key :type "Key Structure"))
  (bind _abilitytwo (`self.AbilityTwo`))
  (:`Pressed`
    (if (`self.CanUseAb2`)
      (bind (_outhit_location _validlocation) (`self.GetMousePositionOnGround`))
      (`/Engine/EditorBlueprintResources/StandardMacros.IsValid` _abilitytwo
        (:`Is Valid`
          (`/Game/Abilities/AbilityBase.Cast` _abilitytwo (`self.K2_GetActorLocation` self) _outhit_location _validlocation (0.0 0.0 0.0) false)
          (set `self.CanUseAb2` false)
          (`KismetSystemLibrary.Delay` (`/Game/Abilities/AbilityBase.Cooldown` _abilitytwo))
          (set `self.CanUseAb2` true))))))

(event `self.DmgComponent.damagedEvent`)

(event `self.DmgComponent.killedEvent`
  (bind _returnvalue (`GameplayStatics.GetPlayerController` 0))
  (`GameplayStatics.SetGamePaused` true)
  (`WidgetBlueprintLibrary.SetInputMode_UIOnlyEx` _returnvalue null)
  (bind _returnvalue_2 (`|CreateWidget` "/Game/EndScreenAssets/DeathScreen.DeathScreen_C" _returnvalue))
  (`WidgetLayoutLibrary.RemoveAllWidgets`)
  (`UserWidget.AddToViewport` _returnvalue_2 0))

(fn `GainAbility`
  (params (AbilityType :type "/Game/Abilities/AbilityBase Class Reference") (DropObject :type "/Game/Abilities/AbilityDrop Object Reference"))
  (bind (_name _description) (defaults `/Game/Blueprints/GrimReaper` AbilityType))
  (bind _returnvalue (`|CreateWidget` "/Game/Abilities/AbilityChoice.AbilityChoice_C" (`GameplayStatics.GetPlayerController` 0)))
  (`/Game/Abilities/AbilityChoice.SetupValues` _returnvalue AbilityType _name _description DropObject)
  (`UserWidget.AddToViewport` _returnvalue 0)
  (`Widget.SetFocus` _returnvalue)
  (`GameplayStatics.SetGamePaused` true))

(fn `GetActorsInCone`
  (params (radius :type "Float (double-precision)") (angle :type "Float (double-precision)") (targetDirection :type "Vector Structure"))
  (returns (Actors :type "Array of Actor Object Reference"))
  (locals (OutArray :type "Array of Actor Object Reference"))
  (bind _returnvalue (/ radius 2.0))
  (bind (_returnvalue_x _returnvalue_y) (`KismetMathLibrary.BreakVector` (`self.K2_GetActorLocation`)))
  (bind _outarray (`local.OutArray`))
  (bind _returnvalue_2 (`KismetMathLibrary.Normal` (- (`KismetMathLibrary.MakeVector` targetDirection_X targetDirection_Y) (`KismetMathLibrary.MakeVector` _returnvalue_x _returnvalue_y))))
  (bind _outactors (`KismetSystemLibrary.BoxOverlapActors` (+ (`self.K2_GetActorLocation`) (* _returnvalue_2 _returnvalue)) (`KismetMathLibrary.GreaterGreater_VectorRotator` (`KismetMathLibrary.MakeVector` _returnvalue angle 1000.0) (`KismetMathLibrary.MakeRotator` 0.0 0.0 (`KismetMathLibrary.Vector_HeadingAngle` _returnvalue_2))) (`|MakeArray` "ObjectTypeQuery3" :!type "EObjectTypeQuery Enum") "/Script/Engine.Actor"))
  (for _array_element _outactors
    (`/Engine/EditorBlueprintResources/StandardMacros.IsValid` (`self.GetComponentByClass` _array_element "/Script/DeathIsTheBeginning.DamageComponent")
      (:`Is Valid`
        (`KismetArrayLibrary.Array_Add` _outarray _array_element))))
  (return _outarray))

(fn `GetMousePositionOnGround`
  (returns (OutHit_Location :type "Vector Structure") (ValidLocation :type Boolean))
  (bind (_worldlocation _worlddirection) (`PlayerController.DeprojectMousePositionToWorld` (`GameplayStatics.GetPlayerController` 0)))
  (bind (_outhit _returnvalue) (`KismetSystemLibrary.LineTraceSingle` (`SceneComponent.K2_GetComponentLocation` (`self.Camera`)) (+ _worldlocation (* _worlddirection 10000.0)) "TraceTypeQuery3"))
  (return (`.Location` (`GameplayStatics.BreakHitResult` _outhit)) _returnvalue))

(fn `Set Ability One`
  (params (AbilityClass :type "/Game/Abilities/AbilityBase Class Reference"))
  (bind _returnvalue (`|GenericCreateObject` AbilityClass self))
  (set `self.AbilityOne` _returnvalue)
  (`KismetSystemLibrary.PrintString` "Ability1 Set"))

(fn `Set Ability Two`
  (params (AbilityClass :type "/Game/Abilities/AbilityBase Class Reference"))
  (bind _returnvalue (`|GenericCreateObject` AbilityClass self))
  (set `self.AbilityTwo` _returnvalue))

(fn `UserConstructionScript`)