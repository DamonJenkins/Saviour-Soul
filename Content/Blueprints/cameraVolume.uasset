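; End-of-level camera volume that plays an exit sequence when the GrimReaper overlaps it, then advances or ends the game.
; Overlap blends the player's view to this actor, snaps the Reaper to the spline component and disables its capsule collision.
; Tick moves and rotates the Reaper along the spline at its max movement speed.
; After the matching delay, it opens Level2 if the current level matches LevelName, otherwise shows EndScreen with UI-only input.
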(event `self.ReceiveActorBeginOverlap`
  (params (OtherActor :type "Actor Object Reference"))
  (bind _returnvalue (`GameplayStatics.GetPlayerController` 0))
  (bind _reaper (`self.reaper`))
  (bind _returnvalue_2 (`GameplayStatics.GetActorOfClass` "/Game/Blueprints/GrimReaper.GrimReaper_C"))
  (if (== _returnvalue_2 OtherActor)
    (set `self.reaper` _returnvalue_2)
    (`PlayerController.SetViewTargetWithBlend` (`GameplayStatics.GetPlayerController` 0) self 2.0 "VTBlend_EaseInOut" 2.0 false)
    (`SceneComponent.K2_SetWorldLocation` (`Character.CapsuleComponent` _reaper) (`SceneComponent.K2_GetComponentLocation` (`self.Spline`)) true false)
    (`PrimitiveComponent.SetCollisionEnabled` (`Character.CapsuleComponent` _reaper) "NoCollision")
    (set `self.onSpline` true)
    (`KismetSystemLibrary.Delay` (/ (`SplineComponent.GetSplineLength` (`self.Spline`)) (`MovementComponent.GetMaxSpeed` (`Character.CharacterMovement` (`self.reaper`)))))
    (bind _returnvalue_3 (`GameplayStatics.GetCurrentLevelName` true))
    (if (`KismetStringLibrary.EqualEqual_StrStr` _returnvalue_3 (`self.levelName`))
      (`GameplayStatics.OpenLevel` "Level2")
      (else
        (bind _returnvalue_4 (`|CreateWidget` "/Game/EndScreenAssets/EndScreen.EndScreen_C" (`GameplayStatics.GetPlayerController` 0)))
        (`UserWidget.AddToViewport` _returnvalue_4 10)
        (set `PlayerController.bShowMouseCursor` true _returnvalue)
        (`WidgetBlueprintLibrary.SetInputMode_UIOnlyEx` _returnvalue _returnvalue_4)))))

(event `self.ReceiveTick`
  (params (DeltaSeconds :type "Float (single-precision)"))
  (bind _spline (`self.Spline`))
  (bind _capsulecomponent (`Character.CapsuleComponent` (`self.reaper`)))
  (if (`self.onSpline`)
    (bind _output_get (set `self.splineDistance` (`KismetMathLibrary.FClamp` (+ (* DeltaSeconds (`MovementComponent.GetMaxSpeed` (`Character.CharacterMovement` (`self.reaper`)))) (`self.splineDistance`)) 0.0 (`SplineComponent.GetSplineLength` _spline))))
    (`SceneComponent.K2_SetWorldLocation` _capsulecomponent (`SplineComponent.GetLocationAtDistanceAlongSpline` _spline _output_get "World") true false)
    (`SceneComponent.K2_SetWorldRotation` _capsulecomponent (`SplineComponent.GetRotationAtDistanceAlongSpline` _spline _output_get "Local") false false)))

(fn `UserConstructionScript`)